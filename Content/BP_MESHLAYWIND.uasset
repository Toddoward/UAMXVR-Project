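; BP_MESHLAYWIND is a wind volume that pushes physics-simulating objects along its up axis.
; Every tick it fires a grid of Visibility traces through the range, applying force at each hit point on simulating components.
; Force blends the up vector with the inverted surface normal, scaled by facing, distance falloff and random variation.
; The construction script sizes the Range box, but its overlap check is disconnected, so traces always run.
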(event EventBeginPlay)

(event Collision|EventActorBeginOverlap
  (params (OtherActor :type Actor%20Object%20Reference)))

(event EventTick
  (params (DeltaSeconds :type Float%20%28single-precision%29))
  (bind _returnvalue (Transformation|GetActorUpVector))
  (bind _returnvalue_2 (Transformation|GetActorTransform))
  (bind _distbetweenforcelines (Variables|Default|GetDistBetweenForceLines))
  (for _index (range 0 (Math|Float|Truncate (/ (Variables|Default|GetrangeX) (Variables|Default|GetDistBetweenForceLines))))
    (for _index_2 (range 0 (Math|Float|Truncate (/ (Variables|Default|GetrangeY) (Variables|Default|GetDistBetweenForceLines))))
      (bind (_outhit _returnvalue_3) (Collision|BoxTraceByChannel (Math|Transform|TransformLocation _returnvalue_2 (Math|Vector|MakeVector (- (* _index_2 _distbetweenforcelines) (/ (Variables|Default|GetrangeX) 2.0)) (- (* _index _distbetweenforcelines) (/ (Variables|Default|GetrangeY) 2.0)) 0.0)) (Math|Transform|TransformLocation _returnvalue_2 (+ (Math|Vector|MakeVector (- (* _index_2 _distbetweenforcelines) (/ (Variables|Default|GetrangeX) 2.0)) (- (* _index _distbetweenforcelines) (/ (Variables|Default|GetrangeY) 2.0)) 0.0) (Math|Vector|MakeVector 0.0 0.0 (Variables|Default|GetrangeZ)))) "0, 0, 0" "0, 0, 0" "TraceTypeQuery1" true 0 "None"))
      (if _returnvalue_3
        (if (Physics|IsSimulatingPhysics (.HitComponent (Collision|BreakHitResult _outhit)) "None")
          (Class|PrimitiveComponent|AddForceatLocation (.HitComponent (Collision|BreakHitResult _outhit)) (* (Math|Vector|Normalize (+ _returnvalue (Math|Vector|NegateVector (.ImpactNormal (Collision|BreakHitResult _outhit))))) (* (Math|Float|Absolute(Float) (Math|Vector|DotProduct _returnvalue (Math|Vector|NegateVector (.ImpactNormal (Collision|BreakHitResult _outhit))))) (+ (* (Variables|Default|GetMaxForce) (- 1.0 (.Time (Collision|BreakHitResult _outhit)))) (* (* (Variables|Default|GetMaxForce) 0.5) (Math|Random|RandomFloat))))) (.ImpactPoint (Collision|BreakHitResult _outhit)) "None"))))))

(fn ConstructionScript
  (Components|Box|SetBoxExtent (Variables|Default|GetRange) (Math|Vector|MakeVector (/ (Variables|Default|GetrangeX) 2.0) (/ (Variables|Default|GetrangeY) 2.0) (/ (Variables|Default|GetrangeZ) 2.0)) true)
  (Transformation|SetRelativeLocation (Variables|Default|GetRange) (Math|Vector|MakeVector 0.0 0.0 (.z (Variables|/Script/Engine.BoxComponent|GetBoxExtent (Variables|Default|GetRange)))) false false))