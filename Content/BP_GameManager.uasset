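; BP_GameManager holds round state for a shape-collecting game: the spawn timer, time remaining and shapes collected count.
; On BeginPlay it resets that state through Restart, then creates the WBP_HUD widget and gives it a reference to itself.
; IncrementShapesCollected raises the count and refreshes the HUD counter text.
; The timers are only initialized here, and the camera setup function is an empty stub.
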(event EventBeginPlay
  (CallFunction|Restart)
  (bind _returnvalue (UserInterface|CreateWidget "/Game/WBP_HUD.WBP_HUD_C"))
  (UserInterface|Viewport|AddtoViewport _returnvalue 0)
  (Variables|/Game/WBP_HUD.WBP_HUD_C|SetGameManager _returnvalue self)
  (bind _output_get (Variables|Default|SetHUBWidget _returnvalue))
  (Default|UpdateCounterText _output_get))

(fn ConstructionScript)

(fn Restart
  (Variables|Default|SetSpawn%20Timer (Variables|Default|GetDuration%20Between%20Spawns))
  (Variables|Default|SetTime%20Remaining (Variables|Default|GetTimer%20Duration))
  (Variables|Default|SetShapes%20Collected 0))

(fn SetUPCamera)

(fn IncrementShapesCollected
  (Math|Integer|IncrementInt (Variables|Default|GetShapes%20Collected)
    (:%20%20
      (Default|UpdateCounterText (Variables|Default|GetHUBWidget)))))